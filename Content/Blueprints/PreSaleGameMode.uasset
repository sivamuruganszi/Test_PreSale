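; PreSale game mode that persists notes data to the PreSaleSave slot and handles quitting the application.
; On BeginPlay it loads any existing save and caches it as SaveFile.
; SaveNotes updates that cached object when the slot exists, or writes a new save object without caching it.
; The quit event always writes the notes into a fresh save object before exiting.
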(event Custom|QuitApplicatiion
  (params (NotesData :type Text))
  ;[1 1 1] Saves notes data and quits the application
  (bind _returnvalue (SaveGame|CreateSaveGameObject "/Game/Blueprints/PreSaleSave.PreSaleSave_C"))
  (Variables|/Game/Blueprints/PreSaleSave.PreSaleSave_C|SetNotesData _returnvalue NotesData)
  (SaveGame|SaveGametoSlot _returnvalue "PreSaleSave")
  (Game|QuitGame 0 "Quit"))

(event Custom|SaveNotes
  (params (NotesData :type Text))
  (bind _savefile (Variables|Default|GetSaveFile))
  ;[1 1 1] Save notes to save file
  (bind _returnvalue (SaveGame|DoesSaveGameExist "PreSaleSave"))
  (if _returnvalue
    (Variables|/Game/Blueprints/PreSaleSave.PreSaleSave_C|SetNotesData _savefile NotesData)
    (SaveGame|SaveGametoSlot _savefile "PreSaleSave")
    (else
      (bind _returnvalue_2 (SaveGame|CreateSaveGameObject "/Game/Blueprints/PreSaleSave.PreSaleSave_C"))
      (Variables|/Game/Blueprints/PreSaleSave.PreSaleSave_C|SetNotesData _returnvalue_2 NotesData)
      (SaveGame|SaveGametoSlot _returnvalue_2 "PreSaleSave"))))

(event EventBeginPlay
  ;[1 1 1] Loads save file object and retrieves the notes text
  (bind _returnvalue (SaveGame|DoesSaveGameExist "PreSaleSave"))
  (if _returnvalue
    (bind _returnvalue_2 (SaveGame|LoadGamefromSlot "PreSaleSave"))
    (bind _aspre_sale_save (Utilities|Casting|CastToPreSaleSave _returnvalue_2))
    (Variables|Default|SetSaveFile _aspre_sale_save)))

(event EventTick
  (params (DeltaSeconds :type Float%20%28single-precision%29)))

(fn ConstructionScript)